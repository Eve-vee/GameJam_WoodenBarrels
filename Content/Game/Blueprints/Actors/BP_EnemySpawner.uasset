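; BP_EnemySpawner is an actor that repeatedly spawns BP_EnemyAI enemies at its own location.
; BeginPlay starts a looping timer at TimeBetweenSpawns that fires SpawnEnemy.
; Each spawn raises Facteur, divides TimeBetweenSpawns by it and prints the result.
; The timer is never re-set, so the changing TimeBetweenSpawns does not alter the actual spawn interval.
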(event Custom|SpawnEnemy
  (Game|SpawnActorfromClass "/Game/Game/Blueprints/Pawns_Characters/Player/BP_EnemyAI.BP_EnemyAI_C" (Math|Transform|MakeTransform (Transformation|GetActorLocation) "0, 0, 0" "1.000000,1.000000,1.000000") "Undefined" "MultiplyWithRoot" 0 0)
  (bind _output_get (Variables|Default|SetFacteur (+ (Variables|Default|GetFacteur) 0.1)))
  (bind _output_get_2 (Variables|Default|SetTimeBetweenSpawns (/ (Variables|Default|GetTimeBetweenSpawns) _output_get)))
  (Development|PrintText (Utilities|Text|FormatText "{Time}" (|GenerictoText _output_get_2))))

(event EventBeginPlay
  (Utilities|Time|SetTimerbyEvent (delegate Custom|SpawnEnemy) (Variables|Default|GetTimeBetweenSpawns) true))

(fn ConstructionScript)