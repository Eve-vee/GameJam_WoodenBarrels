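; Player state Blueprint that owns the player's health component and bridges it to the Game Instance, which can carry health across levels.
; On BeginPlay it loads saved health if the instance's initialized flag is set, otherwise resets health and writes that flag as false.
; Save functions write current and max health to the instance, though nothing here calls them.
; Death opens the death screen level, and a test event deals fixed damage.
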(event OnDeath(AC_Health)
  (Game|OpenLevel(byObjectReference) "/Game/Game/Maps/Lvl_DeathScreen.Lvl_DeathScreen"))

(event Custom|TestDamage
  (Default|TakeDamage (Variables|Default|GetAC_Health) 1e+01))

(event EventBeginPlay
  (bind _asbp_game_instance (Utilities|Casting|CastToBP_GameInstance (Game|GetGameInstance)))
  (bind _output_get (Variables|Default|SetGameInstance%20REF _asbp_game_instance))
  (if (Variables|/Game/Game/Systems/Save_Data/BP_GameInstance.BP_GameInstance_C|GetHealthInitialized_GI _output_get)
    (CallFunction|LoadHealthfromGameInstance)
    (else
      (Default|ResetHealth (Variables|Default|GetAC_Health))
      (Variables|/Game/Game/Systems/Save_Data/BP_GameInstance.BP_GameInstance_C|SetHealthInitialized_GI (Variables|Default|GetGameInstance%20REF) false))))

(fn ConstructionScript)

(fn SaveCurrentHealth
  (params (NewHealth :type Float%20%28double-precision%29))
  (Variables|/Game/Game/Systems/Save_Data/BP_GameInstance.BP_GameInstance_C|SetCurrentHealth_GI (Variables|Default|GetGameInstance%20REF) NewHealth))

(fn SaveMaxHealth
  (params (NewMaxHealth :type Float%20%28double-precision%29))
  (Variables|/Game/Game/Systems/Save_Data/BP_GameInstance.BP_GameInstance_C|SetMaxHealth_GI (Variables|Default|GetGameInstance%20REF) NewMaxHealth))

(fn LoadHealthfromGameInstance
  (bind _ac_health (Variables|Default|GetAC_Health))
  (bind _output_get (Variables|/Game/Game/Blueprints/Components/AC_Health.AC_Health_C|SetMaxHealth (Variables|Default|GetAC_Health) (Variables|/Game/Game/Systems/Save_Data/BP_GameInstance.BP_GameInstance_C|GetMaxHealth_GI (Variables|Default|GetGameInstance%20REF))))
  (bind _output_get_2 (Variables|/Game/Game/Blueprints/Components/AC_Health.AC_Health_C|SetCurrentHealth _ac_health (Variables|/Game/Game/Systems/Save_Data/BP_GameInstance.BP_GameInstance_C|GetCurrentHealth_GI (Variables|Default|GetGameInstance%20REF))))
  (Default|CallOnHealthChanged _ac_health _output_get_2 _output_get))