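; BP_trigger-text is a trigger actor that reveals an in-world text message when the player reaches it.
; Overlap of its Box by BP_ThirdPersonCharacter sets IsVisible and shows the TextRender component.
; The IA_SoulMode input action hides the text when started; leaving the box has no effect.
; An unconnected debug branch with print strings remains in the graph and never runs.
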(event OnComponentBeginOverlap(Box)
  (params (OverlappedComponent :type Primitive%20Component%20Object%20Reference) (OtherActor :type Actor%20Object%20Reference) (OtherComp :type Primitive%20Component%20Object%20Reference) (OtherBodyIndex :type Integer) (bFromSweep :type Boolean) (SweepResult :type Hit%20Result%20Structure%20%28by%20ref%29))
  (Utilities|Casting|CastToBP_ThirdPersonCharacter OtherActor)
  (bind _output_get (Variables|Default|SetisVisible true))
  (Rendering|SetVisibility (Variables|Default|GetTextRender) _output_get false))

(event Input|EnhancedActionEvents|EnhancedInputActionIA_SoulMode
  (params (ActionValue :type Boolean) (ElapsedSeconds :type Float%20%28double-precision%29) (TriggeredSeconds :type Float%20%28double-precision%29) (InputAction :type Input%20Action%20Object%20Reference :default "/Game/Game/Systems/Input/Actions/IA_SoulMode.IA_SoulMode"))
  (:Started
    (bind _output_get (Variables|Default|SetisVisible false))
    (Rendering|SetVisibility (Variables|Default|GetTextRender) _output_get false)))

(event EventBeginPlay)

(event Collision|EventActorBeginOverlap
  (params (OtherActor :type Actor%20Object%20Reference)))

(event EventTick
  (params (DeltaSeconds :type Float%20%28single-precision%29)))

(fn ConstructionScript)